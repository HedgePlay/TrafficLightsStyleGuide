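; Manager actor that cycles all BP_TraffictLight actors through a timed red, yellow, green, yellow sequence, starting on BeginPlay.
; Recolor switches on ColorPicker, finds lights by color tag, applies the CurrentColor entry from the ColorSettings map, then blacks them out after a Delay.
; ColorInc advances index and enum together; the green branch also plays the return yellow and resets to red.
; Recolor calls itself after each branch, looping indefinitely.
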(event `self.ReceiveBeginPlay`
  (`self.Recolor`))

(event `Recolor`
  (bind _colorsettings_colormap (break `/Game/TrafficLightTutorial/Structures/S_LIghtColor` (`self.ColorSettings`)))
  (bind _colorsettings_colormap_2 (break `/Game/TrafficLightTutorial/Structures/S_LIghtColor` (`self.ColorSettings`)))
  (bind _colorsettings_colormap_3 (break `/Game/TrafficLightTutorial/Structures/S_LIghtColor` (`self.ColorSettings`)))
  (bind _colorsettings_colormap_4 (break `/Game/TrafficLightTutorial/Structures/S_LIghtColor` (`self.ColorSettings`)))
  (switch `int` (`self.ColorPicker`)
    (:`Default`
      (bind _outactors (`GameplayStatics.GetAllActorsOfClassWithTag` "/Game/TrafficLightTutorial/Actors/BP_TraffictLight.BP_TraffictLight_C" "Red" :!label _label))
      (`/Game/TrafficLightTutorial/Actors/BP_TraffictLight.ChangeColor` _outactors (`BlueprintMapLibrary.Map_Find` _colorsettings_colormap_2 (`self.CurrentColor`)))
      (`self.ColorInc`)
      (`KismetSystemLibrary.Delay` 5.0)
      (`/Game/TrafficLightTutorial/Actors/BP_TraffictLight.ChangeColor` :`self` _outactors)
      (`self.Recolor`))
    (:`0`
      (goto _label))
    (:`1`
      (bind _outactors_2 (`GameplayStatics.GetAllActorsOfClassWithTag` "/Game/TrafficLightTutorial/Actors/BP_TraffictLight.BP_TraffictLight_C" "Yellow"))
      (`/Game/TrafficLightTutorial/Actors/BP_TraffictLight.ChangeColor` _outactors_2 (`BlueprintMapLibrary.Map_Find` _colorsettings_colormap (`self.CurrentColor`)))
      (`KismetSystemLibrary.Delay` 2.0)
      (`self.ColorInc`)
      (`/Game/TrafficLightTutorial/Actors/BP_TraffictLight.ChangeColor` :`self` _outactors_2)
      (`self.Recolor`))
    (:`2`
      (bind _outactors_3 (`GameplayStatics.GetAllActorsOfClassWithTag` "/Game/TrafficLightTutorial/Actors/BP_TraffictLight.BP_TraffictLight_C" "Green"))
      (`/Game/TrafficLightTutorial/Actors/BP_TraffictLight.ChangeColor` _outactors_3 (`BlueprintMapLibrary.Map_Find` _colorsettings_colormap_3 (`self.CurrentColor`)))
      (set `self.ColorPicker` 1)
      (set `self.CurrentColor` "NewEnumerator1")
      (`KismetSystemLibrary.Delay` 3.0)
      (`/Game/TrafficLightTutorial/Actors/BP_TraffictLight.ChangeColor` :`self` _outactors_3)
      (bind _outactors_4 (`GameplayStatics.GetAllActorsOfClassWithTag` "/Game/TrafficLightTutorial/Actors/BP_TraffictLight.BP_TraffictLight_C" "Yellow"))
      (`/Game/TrafficLightTutorial/Actors/BP_TraffictLight.ChangeColor` _outactors_4 (`BlueprintMapLibrary.Map_Find` _colorsettings_colormap_4 (`self.CurrentColor`)))
      (`KismetSystemLibrary.Delay` 2.0)
      (`self.ColorInc`)
      (`/Game/TrafficLightTutorial/Actors/BP_TraffictLight.ChangeColor` :`self` _outactors_4)
      (set `self.ColorPicker` 0)
      (set `self.CurrentColor` "NewEnumerator0")
      (`self.Recolor`))))

(fn `UserConstructionScript`)